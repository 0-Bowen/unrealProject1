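; Third-person shooter player character with sprint, crouch, prone and jump, in a timed target-dummy shooting mission.
; Right-mouse aiming zooms camera FOV by timeline alongside aim montages, and enables camera line-trace shots that kill TargetDummy actors and count kills.
; Tick drains stamina during fast sprinting, regenerates it otherwise, and fails the mission at 60 counted seconds by disabling input.
; BeginPlay adds stamina and timer widgets and starts looping millisecond timers that build the clock string.
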(event `InputAction|Fire`
  (params (Key :type "Key Structure"))
  (bind _camera (`self.Camera`))
  (bind _returnvalue (`SceneComponent.K2_GetComponentLocation` _camera))
  ;[1 1 1] Shoot
  (:`Pressed`
    (if (`self.RightMousePressed`)
      (`/Engine/EditorBlueprintResources/StandardMacros.IsValid` (`self.rifle`)
        (:`Is Valid`
          (bind _outhit (`KismetSystemLibrary.LineTraceSingle` :`Start` _returnvalue :`End` (+ _returnvalue (* (`SceneComponent.GetForwardVector` _camera) 100000.0)) :`TraceChannel` "TraceTypeQuery1" :`bTraceComplex` true :`DrawDebugType` "ForDuration" :`DrawTime` 1.0))
          (bind (_bblockinghit _binitialoverlap _time _distance _location _impactpoint _normal _impactnormal _physmat _hitactor) (`GameplayStatics.BreakHitResult` _outhit))
          (`KismetSystemLibrary.PrintString` (`KismetSystemLibrary.GetDisplayName` _hitactor))
          (bind _astarget_dummy (cast `/Game/_Project/TargetDummy` _hitactor))
          (`/Game/_Project/TargetDummy.Killed` _astarget_dummy)
          (bind _output_get (set `self.KillCounter` (+ (`self.KillCounter`) 1)))
          (`KismetSystemLibrary.PrintString` (`KismetStringLibrary.Conv_IntToString` _output_get)))))))

(event `millisecond`
  ;[1 1 1] Timer
  (if (not (`self.isPlayer`))
    (set `self.millisecondCount` (+ (`self.millisecondCount`) 1))
    (if (> (`self.millisecondCount`) 999)
      (`/Engine/EditorBlueprintResources/StandardMacros.IncrementInt` (`self.SecondCount`)
        (:`  `
          (set `self.millisecondCount` 0))))))

(event `second`
  ;[1 1 1] Timer
  (set `self.DisplayTimer` "000")
  (if (< (`self.SecondCount`) 10)
    (set `self.DisplayTimer` (`KismetStringLibrary.Concat_StrStr` "00" (`KismetStringLibrary.Conv_IntToString` (`self.SecondCount`))))
    (elif (< (`self.SecondCount`) 100)
      (set `self.DisplayTimer` (`KismetStringLibrary.Concat_StrStr` "0" (`KismetStringLibrary.Conv_IntToString` (`self.SecondCount`))))
      (else
        (set `self.DisplayTimer` (`KismetStringLibrary.Conv_IntToString` (`self.SecondCount`)))))))

(event `ProneToStandAddMovement`
  ;[1 1 1] Bonus
  (`CharacterMovementComponent.SetMovementMode` (`self.CharacterMovement`) "MOVE_Walking" 0))

(event `InputAction|Prone`
  (params (Key :type "Key Structure"))
  ;[1 1 1] prone
  (:`Pressed`
    (set `self.ProneButtonPressed` true)
    (set `self.SprintButtonPressed` false)
    (if (not (`NavMovementComponent.IsFalling` (`self.CharacterMovement`)))
      (`CharacterMovementComponent.SetMovementMode` (`self.CharacterMovement`) "MOVE_None" 0)))
  (:`Released`
    (set `self.ProneButtonPressed` false)))

(event `Key|C`
  (params (Key :type "Key Structure"))
  ;[1 1 1] prone
)

(event `self.ReceiveTick`
  (params (DeltaSeconds :type "Float (single-precision)"))
  ;[1 1 1] Stamina
  (`|ExecutionSequence`
    (:`then_0`
      (if (and (> (`KismetMathLibrary.VSize` (`self.GetVelocity`)) 800.0) (`self.isStamina`) true)
        (set `self.Stamina` (`KismetMathLibrary.FClamp` (- (`self.Stamina`) 0.5) 0.0 100.0))
        (else
          (set `self.Stamina` (`KismetMathLibrary.FClamp` (+ (`self.Stamina`) 1.0) 0.0 100.0)))))
    (:`then_1`
      (if (<= (`self.Stamina`) 0.0)
        (set `self.SprintButtonPressed` false)
        (set `CharacterMovementComponent.MaxWalkSpeed` 600.0 (`self.CharacterMovement`))))
    (:`then_2`
      (`KismetSystemLibrary.Delay` 1.0)
      (`KismetSystemLibrary.PrintString` (`KismetStringLibrary.Conv_DoubleToString` (`KismetMathLibrary.VSize` (`self.GetVelocity`))) true true (struct :`G` 0.66 :`B` 1.0 :`A` 1.0) 1.0))
    (:`then_3`
      ;[1 1 1] Mission Failed
      (if (>= (`self.SecondCount`) 60)
        (`KismetSystemLibrary.PrintString` "MISSION FAILED" true true (struct :`R` 1.0 :`G` 0.155717 :`B` 0.14577 :`A` 1.0) 0.2)
        (`self.DisableInput` null)))))

(event `InputAction|Sprint`
  (params (Key :type "Key Structure"))
  ;[1 1 1] Sprint
  (:`Pressed`
    (if (> (`self.Stamina`) 1.0)
      (if (not (`self.bIsCrouched`))
        (set `self.SprintButtonPressed` true)
        (set `CharacterMovementComponent.MaxWalkSpeed` 900.0 (`self.CharacterMovement`))
        (set `self.isStamina` true)
        (if (`self.RightMousePressed`)
          (`self.StopAnimMontage` "/Game/TPS/AimMontage.AimMontage")
          (`KismetSystemLibrary.PrintString` "set FOV \n")
          (bind (_direction _newtrack_0) (`Timeline|Timeline_0`)
            (:`Update`
              (`CameraComponent.SetFieldOfView` (`self.Camera`) (`KismetMathLibrary.Lerp` (`self.SetFOV`) 90.0 _newtrack_0))))))))
  (:`Released`
    (set `self.SprintButtonPressed` false)
    (set `CharacterMovementComponent.MaxWalkSpeed` 600.0 (`self.CharacterMovement`))
    (set `self.isStamina` false)))

(event `InputAxis|Turn`
  (params (AxisValue :type "Float (single-precision)"))
  ;[1 1 1] Mouse movement
  (`self.AddControllerYawInput` AxisValue))

(event `InputAxis|LookUp`
  (params (AxisValue :type "Float (single-precision)"))
  ;[1 1 1] Mouse movement
  (`self.AddControllerPitchInput` AxisValue))

(event `self.ReceiveBeginPlay`
  ;[1 1 1] widget
  (`self.EnableInput` (`GameplayStatics.GetPlayerController` 0))
  (set `self.SetFOV` (`CameraComponent.FieldOfView` (`self.Camera`)))
  (bind _returnvalue (`|CreateWidget` "/Game/TPS/Staminao.Staminao_C"))
  (bind _returnvalue_2 (`|CreateWidget` "/Game/TPS/TimerBP.TimerBP_C"))
  (`UserWidget.AddToViewport` _returnvalue 0)
  (`UserWidget.AddToViewport` _returnvalue_2 0)
  (`KismetSystemLibrary.K2_SetTimer` null "millisecond" 0.001 true)
  (`KismetSystemLibrary.K2_SetTimer` null "second" 0.001 true))

(event `InputAxis|Sprint`
  (params (AxisValue :type "Float (single-precision)"))
  ;[1 1 1] Movement
  (if (`self.ProneButtonPressed`)
    _
    (elif (not (`self.bIsCrouched`))
      (`self.AddMovementInput` (`KismetMathLibrary.GetForwardVector` (`KismetMathLibrary.MakeRotator` 0.0 0.0 (.yaw (`self.GetControlRotation`)))) AxisValue))))

(event `InputAxis|MoveForward`
  (params (AxisValue :type "Float (single-precision)"))
  ;[1 1 1] Movement
  (if (`self.ProneButtonPressed`)
    _
    (elif (not (`self.SprintButtonPressed`))
      (`self.AddMovementInput` (`KismetMathLibrary.GetForwardVector` (`KismetMathLibrary.MakeRotator` 0.0 0.0 (.yaw (`self.GetControlRotation`)))) (.x (`KismetMathLibrary.Normal` (`KismetMathLibrary.MakeVector` AxisValue (stale `InputAxis|MoveRight` AxisValue))))))))

(event `Key|RightMouseButton`
  (params (Key :type "Key Structure"))
  (bind _camera (`self.Camera`))
  ;[1 1 1] Aim
  (:`Pressed`
    (set `self.RightMousePressed` true)
    (if (not (`self.SprintButtonPressed`))
      (bind (_direction _newtrack_0) (`Timeline|Aim` :!label _label)
        (:`Update`
          (`CameraComponent.SetFieldOfView` _camera (`KismetMathLibrary.Lerp` 90.0 45.0 _newtrack_0))
          (set `self.SetFOV` (`CameraComponent.FieldOfView` _camera))))))
  (:`Released`
    (set `self.RightMousePressed` false)
    (if (not (`self.SprintButtonPressed`))
      (goto _label :!via `Reverse`))))

(event `InputAxis|MoveRight`
  (params (AxisValue :type "Float (single-precision)"))
  ;[1 1 1] Movement
  (if (`self.ProneButtonPressed`)
    _
    (elif (not (`self.SprintButtonPressed`))
      (`self.AddMovementInput` (`KismetMathLibrary.GetRightVector` (`KismetMathLibrary.MakeRotator` 0.0 0.0 (.yaw (`self.GetControlRotation`)))) (.y (`KismetMathLibrary.Normal` (`KismetMathLibrary.MakeVector` (stale `InputAxis|MoveForward` AxisValue) AxisValue)))))))

(event `Key|AnyKey`
  (params (Key :type "Key Structure"))
  ;[1 1 1] Display input Key Names
)

(event `InputAction|Aim`
  (params (Key :type "Key Structure"))
  (bind _mesh (`self.Mesh`))
  ;[1 1 1] Aim
  (:`Pressed`
    (if (`self.SprintButtonPressed`)
      _
      (elif (`self.CrouchButtonPressed`)
        (`|PlayMontage` _mesh "/Game/TPS/AimCrouchMontage.AimCrouchMontage")
        (else
          (`|PlayMontage` _mesh "/Game/TPS/AimMontage.AimMontage")))))
  (:`Released`
    (if (`self.CrouchButtonPressed`)
      (`self.StopAnimMontage` "/Game/TPS/AimCrouchMontage.AimCrouchMontage")
      (else
        (`self.StopAnimMontage` "/Game/TPS/AimMontage.AimMontage")))))

(event `InputAction|Crouch`
  (params (Key :type "Key Structure"))
  (bind _rightmousepressed (`self.RightMousePressed`))
  (bind _mesh (`self.Mesh`))
  ;[1 1 1] Crouch&Aim bug fixing
  (:`Pressed`
    (`self.Crouch`)
    (set `self.CrouchButtonPressed` true)
    (set `self.SprintButtonPressed` false)
    (if _rightmousepressed
      (`|PlayMontage` _mesh "/Game/TPS/AimCrouchMontage.AimCrouchMontage")))
  (:`Released`
    (`self.UnCrouch`)
    (set `self.CrouchButtonPressed` false)
    (if _rightmousepressed
      (`|PlayMontage` _mesh "/Game/TPS/AimMontage.AimMontage"))))

(event `InputAction|Jump`
  (params (Key :type "Key Structure"))
  ;[0.8476 0.2094 1] Jumping
  (:`Pressed`
    (`self.Jump`)
    (set `self.JumpButtonPressed` true))
  (:`Released`
    (`self.StopJumping`)
    (set `self.JumpButtonPressed` false)))

(fn `UserConstructionScript`)