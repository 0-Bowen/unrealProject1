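; Finish point actor for a TPS mission that becomes active once the player character's KillCounter reaches four or more.
; Tick polls that counter every frame, then shows the StaticMesh, Box and TextRender and enables collision on the Box.
; When a TPS_Character_BP overlaps the Box, it sets that character's IsPlayer flag and prints a misspelled mission-accomplished message.
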(event `self.ReceiveTick`
  (params (DeltaSeconds :type "Float (single-precision)"))
  (bind _astps_character_bp (cast `/Game/TPS/TPS_Character_BP` (`GameplayStatics.GetPlayerCharacter` 0)))
  (if (>= (`/Game/TPS/TPS_Character_BP.KillCounter` _astps_character_bp) 4)
    (`SceneComponent.SetVisibility` (`self.StaticMesh`) true true)
    (`SceneComponent.SetVisibility` (`self.Box`) true true)
    (`SceneComponent.SetVisibility` (`self.TextRender`) true true)
    (`PrimitiveComponent.SetCollisionEnabled` (`self.Box`) "QueryAndPhysics")))

(event `self.Box.OnComponentBeginOverlap`
  (params (OverlappedComponent :type "PrimitiveComponent Object Reference") (OtherActor :type "Actor Object Reference") (OtherComp :type "PrimitiveComponent Object Reference") (OtherBodyIndex :type Integer) (bFromSweep :type Boolean) (SweepResult :type "HitResult Structure (by ref)"))
  (bind _astps_character_bp (cast `/Game/TPS/TPS_Character_BP` OtherActor))
  (set `/Game/TPS/TPS_Character_BP.isPlayer` true _astps_character_bp)
  (`KismetSystemLibrary.PrintString` "Mission Acocmpolsh"))

(fn `UserConstructionScript`)