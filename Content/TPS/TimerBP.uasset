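; Timer Blueprint that shows a Timer widget on screen and keeps a running count of elapsed time.
; BeginPlay creates the widget and adds it to the viewport.
; Tick uses a 0.1-second Delay to throttle increments of TimeMSec, which bumps TimeSec and resets once it exceeds 10, so each counted second spans eleven increments.
; A game-time debug print is left unconnected.
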(event `self.ReceiveBeginPlay`
  (bind _returnvalue (`|CreateWidget` "/Game/TPS/Timer.Timer_C"))
  (`UserWidget.AddToViewport` _returnvalue 0))

(event `self.ReceiveTick`
  (params (DeltaSeconds :type "Float (single-precision)"))
  (`KismetSystemLibrary.Delay` 0.1)
  (set `self.Time_MSec` (+ (`self.Time_MSec`) 1))
  (if (> (`self.Time_MSec`) 10)
    (set `self.Time_Sec` (+ (`self.Time_Sec`) 1))
    (set `self.Time_MSec` 0)))

(fn `UserConstructionScript`)