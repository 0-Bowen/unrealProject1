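; BP_Enemys is an enemy actor that turns to face the player while it is alive.
; Each Tick, it applies only the yaw of a look-at rotation toward player character 0, keeping pitch and roll at zero.
; Die clears the Alive flag, which stops the turning.
; Tick also runs a debug print of Alive through a two-second Delay.
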(event `self.ReceiveTick`
  (params (DeltaSeconds :type "Float (single-precision)"))
  (bind _alive (`self.Alive`))
  (`|ExecutionSequence`
    (:`then_0`
      (if _alive
        (`self.K2_SetActorRotation` (`KismetMathLibrary.MakeRotator` 0.0 0.0 (.yaw (`KismetMathLibrary.FindLookAtRotation` (`self.K2_GetActorLocation`) (`self.K2_GetActorLocation` (`GameplayStatics.GetPlayerCharacter` 0))))))))
    (:`then_1`
      (`KismetSystemLibrary.Delay` 2.0)
      (`KismetSystemLibrary.PrintString` (`KismetStringLibrary.Conv_BoolToString` _alive) true true (struct :`G` 0.66 :`B` 1.0 :`A` 1.0) 1.0))))

(fn `Die`
  (set `self.Alive` false))

(fn `UserConstructionScript`)