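; BP_Enemy is an enemy actor that turns to face the player character while it is alive.
; Each Tick it computes a look-at rotation to player 0 and applies only the yaw, so the actor stays upright.
; When its skeletal mesh hits another BP_Enemy, it stores that actor in the Enemy variable, which nothing in this graph reads.
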(event `self.ReceiveTick`
  (params (DeltaSeconds :type "Float (single-precision)"))
  (if (`self.Alive`)
    (`self.K2_SetActorRotation` (`KismetMathLibrary.MakeRotator` 0.0 0.0 (.yaw (`KismetMathLibrary.FindLookAtRotation` (`self.K2_GetActorLocation`) (`self.K2_GetActorLocation` (`GameplayStatics.GetPlayerCharacter` 0))))))))

(event `self.SkeletalMesh.OnComponentHit`
  (params (HitComponent :type "PrimitiveComponent Object Reference") (OtherActor :type "Actor Object Reference") (OtherComp :type "PrimitiveComponent Object Reference") (NormalImpulse :type "Vector Structure") (Hit :type "HitResult Structure (by ref)"))
  (bind _asbp_enemy (cast `/Game/_Project/BP_Enemy` OtherActor))
  (set `self.Enemy` _asbp_enemy))

(fn `UserConstructionScript`)